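; BP_Jordan is a player character Blueprint with walking, sprinting, jumping and look controls.
; BeginPlay adds the IMC_Default Enhanced Input mapping context for the controlling player.
; Move input follows the actor's forward and right vectors, look drives controller yaw and pitch, and jump uses the built-in Jump and StopJumping.
; Sprint raises max walk speed when started and lowers it only on Canceled, with no Completed handler.
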(event `self.ReceiveBeginPlay`
  (bind _asplayer_controller (cast `PlayerController` (`self.GetController`)))
  (bind _returnvalue (pcsubsystem `EnhancedInputLocalPlayerSubsystem` _asplayer_controller))
  (`/Engine/EditorBlueprintResources/StandardMacros.IsValid` _returnvalue
    (:`Is Valid`
      (`EnhancedInputSubsystemInterface.AddMappingContext` _returnvalue "/Game/Player/Input/IMC_Default.IMC_Default" 0 (struct)))))

(event `EnhancedInput|/Game/Player/Input/Actions/IA_Sprint`
  (params (ActionValue :type Boolean) (ElapsedSeconds :type "Float (double-precision)") (TriggeredSeconds :type "Float (double-precision)") (InputAction :type "InputAction Object Reference" :default "/Game/Player/Input/Actions/IA_Sprint.IA_Sprint"))
  (bind _charactermovement (`self.CharacterMovement`))
  (:`Started`
    (set `CharacterMovementComponent.MaxWalkSpeed` 400.0 _charactermovement))
  (:`Canceled`
    (set `CharacterMovementComponent.MaxWalkSpeed` 150.0 _charactermovement)))

(event `EnhancedInput|/Game/Player/Input/Actions/IA_Move`
  (params (ActionValue :type "Vector2D Structure") (ElapsedSeconds :type "Float (double-precision)") (TriggeredSeconds :type "Float (double-precision)") (InputAction :type "InputAction Object Reference" :default "/Game/Player/Input/Actions/IA_Move.IA_Move"))
  (:`Triggered`
    (`self.AddMovementInput` (`self.GetActorRightVector`) ActionValue_X)
    (`self.AddMovementInput` (`self.GetActorForwardVector`) ActionValue_Y)))

(event `EnhancedInput|/Game/Player/Input/Actions/IA_Jump`
  (params (ActionValue :type Boolean) (ElapsedSeconds :type "Float (double-precision)") (TriggeredSeconds :type "Float (double-precision)") (InputAction :type "InputAction Object Reference" :default "/Game/Player/Input/Actions/IA_Jump.IA_Jump"))
  (:`Started`
    (`self.Jump`))
  (:`Completed`
    (`self.StopJumping`)))

(event `EnhancedInput|/Game/Player/Input/Actions/IA_Look`
  (params (ActionValue :type "Vector2D Structure") (ElapsedSeconds :type "Float (double-precision)") (TriggeredSeconds :type "Float (double-precision)") (InputAction :type "InputAction Object Reference" :default "/Game/Player/Input/Actions/IA_Look.IA_Look"))
  (:`Triggered`
    (`self.AddControllerYawInput` ActionValue_X)
    (`self.AddControllerPitchInput` ActionValue_Y)))

(fn `UserConstructionScript`)